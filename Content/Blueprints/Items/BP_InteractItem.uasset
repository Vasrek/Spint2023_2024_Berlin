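; BP_InteractItem is an interactable item that registers itself with the player when they come within range.
; On Box begin overlap, unless DoNotInteractAnyomore is set, it shows its name and type on the player's HUD and sets itself as BP_Player's InteractItem.
; On end overlap, it hides the HUD widget and clears that reference.
; The interaction itself is not implemented in these graphs.
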(event OnComponentBeginOverlap(Box)
  (params (OverlappedComponent :type Primitive%20Component%20Object%20Reference) (OtherActor :type Actor%20Object%20Reference) (OtherComp :type Primitive%20Component%20Object%20Reference) (OtherBodyIndex :type Integer) (bFromSweep :type Boolean) (SweepResult :type Hit%20Result%20Structure%20%28by%20ref%29))
  (if (not (Variables|Default|GetDoNotInteractAnyomore))
    (bind _asbp_player (Utilities|Casting|CastToBP_Player OtherActor))
    (Default|UpdateInteractText (Variables|/Game/Blueprints/Player/BP_Player.BP_Player_C|GetHUDReference _asbp_player) (Variables|ItemInfo|GetNameItem) (Variables|ItemInfo|GetInteractItemType))
    (Variables|/Game/Blueprints/Player/BP_Player.BP_Player_C|SetInteractItem _asbp_player self)))

(event OnComponentEndOverlap(Box)
  (params (OverlappedComponent :type Primitive%20Component%20Object%20Reference) (OtherActor :type Actor%20Object%20Reference) (OtherComp :type Primitive%20Component%20Object%20Reference) (OtherBodyIndex :type Integer))
  (bind _asbp_player (Utilities|Casting|CastToBP_Player OtherActor))
  (Default|HideWidget (Variables|/Game/Blueprints/Player/BP_Player.BP_Player_C|GetHUDReference _asbp_player))
  (Variables|/Game/Blueprints/Player/BP_Player.BP_Player_C|SetInteractItem _asbp_player 0))

(fn ConstructionScript)